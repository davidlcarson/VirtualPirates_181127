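; First-person player character that can sprint and board or leave boats.
; Boat triggers set the nearby-boat flag and pointer; pressing EnterExitBoat then notifies that boat and hands controller possession to it, hiding the character and disabling its collision.
; VacateBoat restores the character at a supplied transform, keeping only yaw rotation, and repossesses it.
; In-boat state and boat ID are tracked for save/load routines.
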(event EventBeginPlay)

(event Collision|EventActorBeginOverlap
  (params (OtherActor :type Actor%20Object%20Reference)))

(event EventTick
  (params (DeltaSeconds :type Float%20%28single-precision%29)))

(event Input|ActionEvents|InputActionEnterExitBoat
  (params (Key :type Key%20Structure))
  (:Pressed
    (if (not (Variables|Default|GetbInBoat))
      (if (Variables|Default|GetbNearBoat)
        (Default|Boarded (Variables|Default|GetpNearBoat) self) ; BOat Routine
        (CallFunction|OccupyBoat) ; Our routine
      ))))

(event Input|ActionEvents|InputActionSprint
  (params (Key :type Key%20Structure))
  (bind _charactermovement (Variables|Character|GetCharacterMovement))
  (bind _mymaxwalkspeed (Variables|Default|GetMyMaxWalkSpeed))
  ;[1 1 1] Sprint
  (:Pressed
    (Variables|/Script/Engine.CharacterMovementComponent|SetMaxWalkSpeed _charactermovement (* _mymaxwalkspeed 6.0)))
  (:Released
    (Variables|/Script/Engine.CharacterMovementComponent|SetMaxWalkSpeed _charactermovement _mymaxwalkspeed)))

(fn ConstructionScript)

(fn SetNearBoat
  (params (bNearBoat :type Boolean) (pBoatWereNear :type BPD%20Boat%20Locator%20Pawn%20Object%20Reference))
  ;[1 1 1] Called by Boat Locator whenever MyFPChar begins or ends overlap w/ trigger. Sets 'near' flag and sets pointer to boat we're near
  (Variables|Default|SetbNearBoat bNearBoat)
  (Variables|Default|SetpNearBoat pBoatWereNear) ; This is boat we're near (will be NULL if exiting trigger)
)

(fn OccupyBoat
  (Variables|Default|SetpBoatWereIn (Variables|Default|GetpNearBoat))
  ;[1 1 1] This is for saving/loading routines
  (Variables|Default|SetbInBoat true)
  (Variables|Default|SetBoatID (Variables|/Script/VIrtPirates_181127.CPC_Boat_Locator_Pawn|GetBoatID (Variables|Default|GetpBoatWereIn)))
  (Pawn|Possess (Game|GetPlayerController 0) (Variables|Default|GetpNearBoat)) ; Controller Possesses the Boat Locator
  ;[1 1 1] We're in boat - Hide Player
  (Rendering|SetActorHiddenInGame true) ; MyFP Needs to be invisible now
  (Collision|SetActorEnableCollision false) ; Can't run into MY FP
)

(fn VacateBoat
  (params (PlayerTransform :type Transform))
  (bind (_location _rotation _scale) (Math|Transform|BreakTransform PlayerTransform))
  (if (Variables|Default|GetbInBoat)
    (Variables|Default|SetbInBoat false)
    (Variables|Default|SetbNearBoat false)
    (Variables|Default|SetBoatID -1)
    (Transformation|SetActorTransform (Math|Transform|MakeTransform _location (Math|Rotator|MakeRotator 0.0 0.0 (.Yaw (Math|Rotator|BreakRotator _rotation))) _scale))
    (Rendering|SetActorHiddenInGame false)
    (Collision|SetActorEnableCollision true)
    (Pawn|Possess (Pawn|GetController (Variables|Default|GetpBoatWereIn)) self) ; Re-Possess the FP Character
  ))