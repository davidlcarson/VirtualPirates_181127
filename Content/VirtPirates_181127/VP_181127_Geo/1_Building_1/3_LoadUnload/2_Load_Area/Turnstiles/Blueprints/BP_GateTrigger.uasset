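; Trigger actor that animates an array of turnstiles when a boat locator pawn enters its GateCollision volume, in the load/unload area.
; The overlap resets a timer and sets an animating flag, ignoring new overlaps until the animation finishes.
; While flagged, Tick samples a float curve and passes the value to each turnstile's RotateFlaps.
; At the curve's end time, it snaps the flaps to zero and clears the flag.
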(event OnComponentBeginOverlap(GateCollision)
  (params (OverlappedComponent :type Primitive%20Component%20Object%20Reference) (OtherActor :type Actor%20Object%20Reference) (OtherComp :type Primitive%20Component%20Object%20Reference) (OtherBodyIndex :type Integer) (bFromSweep :type Boolean) (SweepResult :type Hit%20Result%20Structure%20%28by%20ref%29))
  (Utilities|Casting|CastToBPD_Boat_Locator_Pawn OtherActor)
  ;[1 1 1] Flag gate as animating
  (if (Variables|Default|GetbGatesAnimating) ; Ignore if gates are open
    (Development|PrintString "Gates Already Animating")
    (else
      (Variables|Default|SetbGatesAnimating true)
      ;[1 1 1] Reset timer.
      (Variables|Default|SetelapsedTime 0.0))))

(event EventBeginPlay
  ;[1 1 1] Store duration of animation
  (Variables|Default|SetEndTime (.MaxTime (Math|Curves|GetTimeRange (Variables|Default|GetTurnstileCurve)))))

(event Collision|EventActorBeginOverlap
  (params (OtherActor :type Actor%20Object%20Reference)))

(event EventTick
  (params (DeltaSeconds :type Float%20%28single-precision%29))
  (if (Variables|Default|GetbGatesAnimating) ; Execute this routine whenever gates are animating
    ;[1 1 1] Read data from curves - store locally
    (bind _output_get (Variables|Default|SetelapsedTime (+ DeltaSeconds (Variables|Default|GetelapsedTime)))) ; Update elapsed animation time
    (bind _output_get_2 (Variables|Default|SetlocRotationValue (Math|Curves|GetFloatValue (Variables|Default|GetTurnstileCurve) _output_get)))
    (for _array_element (Variables|Default|GetTurnstyle_array)
      (Default|RotateFlaps _array_element _output_get_2)
      (if (>= (Variables|Default|GetelapsedTime) (Variables|Default|GetEndTime)) ; are we done animating?
        (Default|RotateFlaps _array_element 0.0) ; CLear any inaccuracy
        (Variables|Default|SetbGatesAnimating false) ; Done. Clear 'animating' flag
      ))))

(fn ConstructionScript)