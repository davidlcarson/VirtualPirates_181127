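; Boat trigger volume that drives a timed speed and bobbing change on the boat whose locator pawn overlaps it.
; Overlap stores the boat ID and starts a timer; Tick samples SpeedCurve and BobCurve and sends both rates to the Armada until the speed curve ends.
; A new overlap within two seconds restarts the animation, while a later one mid-animation pauses the Armada and prints a warning.
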(event OnComponentBeginOverlap(CollisionComponent)
  (params (OverlappedComponent :type Primitive%20Component%20Object%20Reference) (OtherActor :type Actor%20Object%20Reference) (OtherComp :type Primitive%20Component%20Object%20Reference) (OtherBodyIndex :type Integer) (bFromSweep :type Boolean) (SweepResult :type Hit%20Result%20Structure%20%28by%20ref%29))
  ;[1 1 1] Overlapping w/ Boat Trigger?
  (bind _asbpd_boat_locator_pawn (Utilities|Casting|CastToBPD_Boat_Locator_Pawn OtherActor))
  ;[1 1 1] Already animating?
  (if (Variables|Default|GetbAnimating)
    ;[1 1 1] True: More than 2 seconds?
    (if (> (Variables|Default|GetElapsedTime) 2.0) ; More than 2 secs?
      ;[1 1 1] true = 2nd boat in trigger. Pause Armada
      (Default|PauseArmada (Variables|Default|GetArmada_ref) true)
      (Development|PrintString (Utilities|String|Append "Second Boat in Trigger " (Utilities|String|ToString(Integer) (Variables|Default|GetTriggerID)))) ; 2nd Boat Entering while animating!!
      (else
        ;[1 1 1] false = Start Animation
        (Variables|Default|Setloc_boatID (Variables|/Script/VIrtPirates_181127.CPC_Boat_Locator_Pawn|GetBoatID _asbpd_boat_locator_pawn) :!label _label)
        (Variables|Default|SetElapsedTIme 0.0)
        (Variables|Default|SetbAnimating true)))
    (else
      (goto _label))))

(event EventBeginPlay
  ;[1 1 1] Store duration of animation
  (Variables|Default|SetEndTime (.MaxTime (Math|Curves|GetTimeRange (Variables|Default|GetSpeedCurve)))))

(event EventTick
  (params (DeltaSeconds :type Float%20%28single-precision%29))
  ;[1 1 1] Are we animating?
  (if (Variables|Default|GetbAnimating)
    (Variables|Default|SetElapsedTIme (+ DeltaSeconds (Variables|Default|GetElapsedTIme))) ; Update Elapsed Time
    ;[1 1 1] Read data from curves - store locally
    (Variables|Default|Setloc_speedFactor (Math|Curves|GetFloatValue (Variables|Default|GetSpeedCurve) (Variables|Default|GetElapsedTIme))) ; Store speed-rate from curve locally
    (bind _output_get (Variables|Default|Setloc_bobFactor (Math|Curves|GetFloatValue (Variables|Default|GetBobCurve) (Variables|Default|GetElapsedTIme)))) ; Store bob-rate from curve locally
    ;[1 1 1] Send data to Armada for conversion
    (Class|CPCArmada|SetBoatAnimbyRate (Variables|Default|GetArmada_ref) (Variables|Default|Getloc_boatID) (Variables|Default|Getloc_speedFactor) (Variables|Default|Getloc_bobFactor))
    ;[1 1 1] Test for End of Animation curve
    (if (>= (Variables|Default|GetElapsedTime) (Variables|Default|GetEndTime)) ; Are we at end of animation?
      (Variables|Default|SetbAnimating false))))

(fn ConstructionScript)